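; Game instance Blueprint that handles PlayFab account registration and email login for the game's menus.
; Init sets the PlayFab title ID, and two events send registration and login requests from supplied credentials.
; Successful registration opens the InicioSesion widget, while successful login opens Seleccion_Usuario.
; Registration failures print the error in red on screen.
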(event `self.ReceiveInit`
  (`PlayFabUtilities.setPlayFabSettings` "2A987"))

(event `OnSuccess`
  (params (result :type "ClientRegisterPlayFabUserResult Structure") (customData :type "Object Object Reference"))
  (`GameplayStatics.GetActorOfClass` "/Game/Blueprints/personaje.personaje_C")
  (bind _returnvalue (`|CreateWidget` "/Game/Menu/Widgets/InicioSesion.InicioSesion_C"))
  (`UserWidget.AddToViewport` _returnvalue 0))

(event `/Game/Menu/BI_GameInterface.RegistroPlayfab`
  (params (Username :type Text) (Email :type Text) (Password :type Text))
  (`PlayFabClientAPI.RegisterPlayFabUser` (make `ClientRegisterPlayFabUserRequest` :`Email` (`KismetTextLibrary.Conv_TextToString` Email) :`Password` (`KismetTextLibrary.Conv_TextToString` Password) :`Username` (`KismetTextLibrary.Conv_TextToString` Username)) (delegate `OnSuccess`) (delegate `OnFail`)))

(event `OnFail`
  (params (error :type "PlayFabError Structure") (customData :type "Object Object Reference"))
  (`KismetSystemLibrary.PrintString` (`KismetStringLibrary.Concat_StrStr` error_ErrorName ":" error_ErrorMessage "(" error_ErrorDetails ").") true true (struct :`R` 1.0 :`G` 0.011436 :`A` 1.0) 10.0))

(event `/Game/Menu/BI_GameInterface.LoginPlayfab`
  (params (Email :type Text) (Password :type Text))
  (`PlayFabClientAPI.LoginWithEmailAddress` (make `ClientLoginWithEmailAddressRequest` null (`KismetTextLibrary.Conv_TextToString` Email) null (`KismetTextLibrary.Conv_TextToString` Password)) (delegate `LoginSuccess`) (`|CreateDelegate` :!event `OnFail`)))

(event `LoginSuccess`
  (params (result :type "ClientLoginResult Structure") (customData :type "Object Object Reference"))
  (bind _returnvalue (`|CreateWidget` "/Game/Menu/Widgets/Seleccion_Usuario.Seleccion_Usuario_C"))
  (`UserWidget.AddToViewport` _returnvalue 0))