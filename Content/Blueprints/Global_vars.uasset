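; Global_vars is a global Blueprint, apparently a GameInstance, that handles PlayFab accounts and a shared list of place names.
; Init sets the PlayFab title ID; registration success opens the InicioSesion widget, while failure prints the error on screen.
; Email login chains into an account-info request, storing the display name and opening the Seleccion_Usuario widget.
; LlenarListaLugares rebuilds ListaLugares from every Lugar in the Bloques of Personaje's current Sede.
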(event `self.ReceiveInit`
  (`PlayFabUtilities.setPlayFabSettings` "5A199"))

(event `OnFail`
  (params (error :type "PlayFabError Structure") (customData :type "Object Object Reference"))
  (`KismetSystemLibrary.PrintString` (`KismetStringLibrary.Concat_StrStr` error_ErrorName ":" error_ErrorMessage "(" error_ErrorDetails ").") true true (struct :`R` 1.0 :`G` 0.011436 :`A` 1.0) 10.0))

(event `OnSuccess`
  (params (result :type "ClientRegisterPlayFabUserResult Structure") (customData :type "Object Object Reference"))
  (`GameplayStatics.GetActorOfClass` "/Game/Blueprints/personaje.personaje_C")
  (bind _returnvalue (`|CreateWidget` "/Game/Menu/Widgets/InicioSesion.InicioSesion_C"))
  (`UserWidget.AddToViewport` _returnvalue 0))

(event `/Game/Menu/BI_GameInterface.RegistroPlayfab`
  (params (Username :type Text) (Email :type Text) (Password :type Text))
  (bind _returnvalue (`KismetTextLibrary.Conv_TextToString` Username))
  (`PlayFabClientAPI.RegisterPlayFabUser` (make `ClientRegisterPlayFabUserRequest` null _returnvalue (`KismetTextLibrary.Conv_TextToString` Email) "" null (`KismetTextLibrary.Conv_TextToString` Password) "" false _returnvalue) (delegate `OnSuccess`) (delegate `OnFail`)))

(event `CustomEvent_0`
  (params (result :type "ClientGetAccountInfoResult Structure") (customData :type "Object Object Reference"))
  (set `self.usernameplayer` (`PlayFabJsonObject.GetStringField` (`PlayFabJsonObject.GetObjectField` (`.AccountInfo` (break `ClientGetAccountInfoResult` result)) "TitleInfo") "Displayname"))
  (`GameplayStatics.GetActorOfClass` "/Game/Blueprints/personaje.personaje_C")
  (bind _returnvalue (`|CreateWidget` "/Game/Menu/Widgets/Seleccion_Usuario.Seleccion_Usuario_C"))
  (`UserWidget.AddToViewport` _returnvalue 0))

(event `LoginSuccess`
  (params (result :type "ClientLoginResult Structure") (customData :type "Object Object Reference"))
  (`PlayFabClientAPI.GetAccountInfo` (make `ClientGetAccountInfoRequest` "" (`.PlayFabId` (break `ClientLoginResult` result))) (delegate `CustomEvent_0`) (`|CreateDelegate` :!event `OnFail`)))

(event `/Game/Menu/BI_GameInterface.LoginPlayfab`
  (params (Email :type Text) (Password :type Text))
  (`PlayFabClientAPI.LoginWithEmailAddress` (make `ClientLoginWithEmailAddressRequest` null (`KismetTextLibrary.Conv_TextToString` Email) null (`KismetTextLibrary.Conv_TextToString` Password)) (delegate `LoginSuccess`) (`|CreateDelegate` :!event `OnFail`)))

(fn `Llenar_lista_lugares`
  (`KismetArrayLibrary.Array_Clear` (`self.Lista_lugares`))
  (bind _returnvalue (`GameplayStatics.GetActorOfClass` "/Game/Blueprints/personaje.personaje_C"))
  (for _array_element (`/Game/Blueprints/Sede.Bloques` (`/Game/Blueprints/personaje.Sede_actual` _returnvalue))
    (for _array_element_2 (`/Game/Blueprints/Bloque.Lugares` _array_element)
      (`KismetArrayLibrary.Array_Add` (`self.Lista_lugares`) (`/Game/Blueprints/Lugar.Nombre_lugar` _array_element_2)))))